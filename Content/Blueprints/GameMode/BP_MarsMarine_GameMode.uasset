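; Game mode for Mars Marine that continuously spawns aliens into the level.
; After a short delay on BeginPlay, it increments CurrentWave once and starts a looping timer that fires SpawnWave.
; Each tick of that timer calls SpawnAlien, which spawns one BP_Alien at the transform of a randomly chosen TargetPoint actor.
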(event `self.ReceiveBeginPlay`
  (`KismetSystemLibrary.Delay` 2.0)
  (`/Engine/EditorBlueprintResources/StandardMacros.IncrementInt` (`self.Current Wave`)
    (:`  `
      (`KismetSystemLibrary.K2_SetTimerDelegate` (delegate `Spawn Wave`) 1.0 true))))

(event `Spawn Wave`
  (`self.Spawn Alien`))

(fn `Spawn Alien`
  (bind _outactors (`GameplayStatics.GetAllActorsOfClass` "/Script/Engine.TargetPoint"))
  (`|SpawnActorFromClass` "/Game/Blueprints/AI/BP_Alien.BP_Alien_C" (`self.GetTransform` (`KismetArrayLibrary.Array_Random` _outactors)) "Undefined" "MultiplyWithRoot" null null))

(fn `UserConstructionScript`)